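; BP_SplineTool is an editor-placed spline tool that populates spline mesh components at regular intervals along its spline.
; The construction script divides spline length by SplineSpacing, then adds a component at each step using the world-space location and rotation as its relative transform.
; Every component's start and end both use spline point 0's local position and tangent, so segments do not follow successive points.
; The event graph has no active logic.
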(fn `UserConstructionScript`
  (bind _spline (`self.Spline`))
  (bind _splinespacing (`self.SplineSpacing`))
  (bind _spline_2 (`self.Spline`))
  (bind (_location _tangent) (`SplineComponent.GetLocationAndTangentAtSplinePoint` _spline_2 0 "Local"))
  (bind (_location_2 _tangent_2) (`SplineComponent.GetLocationAndTangentAtSplinePoint` _spline_2 0 "Local"))
  (for _index (range (+ (`.ReturnValue` (`KismetMathLibrary.FMod` (`SplineComponent.GetSplineLength` _spline) _splinespacing)) 1))
    (bind _returnvalue (* _index _splinespacing))
    (bind _returnvalue_2 (`AddComponent|NODE_AddSplineMeshComponent-0` :`RelativeTransform` (`KismetMathLibrary.MakeTransform` (`SplineComponent.GetLocationAtDistanceAlongSpline` _spline _returnvalue "World") (`SplineComponent.GetRotationAtDistanceAlongSpline` _spline _returnvalue "World"))))
    (`SplineMeshComponent.SetStartAndEnd` _returnvalue_2 _location_2 _tangent_2 _location _tangent true)))