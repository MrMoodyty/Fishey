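; Actor component for a fishing lure that tracks whether it is in a fishing volume, apparently groundwork for buoyancy.
; BeginPlay caches the owner through its FishingLureMessage cast and starts a looping timer on UpdateBouyancy.
; UpdateFishingVolumeParm stores the in-volume flag and entry point.
; UpdateBouyancy is currently empty; the depth-scaled upward force math sits disconnected, so no buoyancy is applied.
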(event `self.ReceiveBeginPlay`
  (bind _fishinglure (message `/Game/Tyler/BluePrints/FishingFeature/BPI_FIshingLure.AsFishingLure` (`self.GetOwner`)))
  (set `self.Fishing Lure` _fishinglure)
  (bind _returnvalue (`KismetSystemLibrary.K2_SetTimerDelegate` (delegate `UpdateBouyancy`) (`self.UpdateTime`) true))
  (set `self.TimerHandle` _returnvalue))

(event `UpdateBouyancy`)

(fn `UpdateFishingVolumeParm`
  (params (IsInFishingVolume :type Boolean) (InputPin :type "Vector Structure"))
  (set `self.IsInFishingVolume` IsInFishingVolume)
  (set `self.FishingVolumeEntryPoint` InputPin))