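; Fishing component for the third-person character that casts a lure from the rod's line socket using the CastingPole input action.
; Starting the input destroys any existing lure, and holding it maps the elapsed time to a clamped throw strength.
; Completing or canceling spawns a new lure oriented from the camera's forward vector, with speed scaled by that strength.
; A cable component added to the lure at runtime draws the line back to the socket.
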(event `self.ReceiveBeginPlay`
  (bind _asthirdpersoncharacter (message `/Game/Tyler/BluePrints/FishingFeature/BPI_Fishing.As Third Person Character` (`self.GetOwner`)))
  (set `self.As Third Person Character` _asthirdpersoncharacter))

(event `EnhancedInput|/Game/Tyler/Inputs/CastingPole_IA`
  (params (ActionValue :type Boolean) (ElapsedSeconds :type "Float (double-precision)") (TriggeredSeconds :type "Float (double-precision)") (InputAction :type "InputAction Object Reference" :default "/Game/Tyler/Inputs/CastingPole_IA.CastingPole_IA"))
  (bind _as_third_person_character (`self.As Third Person Character`))
  (bind _fishinglureobjref (`self.FishingLureOBJRef`))
  (bind _returnvalue (`self.GetSocketLocation` (`self.FishingLineSocket`)))
  (:`Started`
    (`/Engine/EditorBlueprintResources/StandardMacros.IsValid` _fishinglureobjref
      (:`Is Valid`
        (`Actor.K2_DestroyActor` _fishinglureobjref))))
  (:`Ongoing`
    (set `self.ThrowStrength` (`KismetMathLibrary.MapRangeClamped` ElapsedSeconds 0.0 0.0 (`self.MinThrowStrength`) (`self.MaxThrowStrength`))))
  (:`Canceled`
    (bind _returnvalue_2 (`|SpawnActorFromClass` (`self.FishingLureRef`) (`KismetMathLibrary.MakeTransform` _returnvalue (`KismetMathLibrary.MakeRotFromXY` (`self.GetForwardVector` (`/Game/Tyler/BluePrints/ThirdPersonCharacter_BP.Camera` (`self.As Third Person Character`))) _returnvalue)) "Undefined" "MultiplyWithRoot" _as_third_person_character (* (`self.ThrowStrength`) (`self.FishingLureBaseSpeed`)) _as_third_person_character :!label _label))
    (bind _output_get (set `self.FishingLureOBJRef` _returnvalue_2))
    (bind _returnvalue_3 (`|AddComponentByClass` :`self` _output_get :`Class` (`self.FishingRodLine`)))
    (`self.SetMaterial` _returnvalue_3 0 "/Engine/MapTemplates/Materials/BasicAsset03.BasicAsset03")
    (set `CableComponent.CableWidth` 5.0 _returnvalue_3)
    (`CableComponent.SetAttachEndToComponent` _returnvalue_3 self (`self.FishingLineSocket`))
    (set `CableComponent.EndLocation` (0.0 0.0 0.0) _returnvalue_3)
    (`self.SetVisibility` _returnvalue_3 true true))
  (:`Completed`
    (goto _label)))