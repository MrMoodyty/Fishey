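; Inventory component for a fishing game that stores general items, fish, lures and baits in separate collections.
; Each category has its own add function that appends the new item to its collection and prints it for debugging.
; The fish and bait removal functions are empty stubs, and BeginPlay and Tick are unused.
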(fn `AddBaitToInventory`
  (params (NewItem :type String))
  (`KismetArrayLibrary.Array_Add` (`self.Baits`) NewItem)
  (`KismetSystemLibrary.PrintString` NewItem))

(fn `AddFishToInventory`
  (params (NewItem :type "String (by ref)"))
  (`KismetArrayLibrary.Array_Add` (`self.Fish`) NewItem)
  (`KismetSystemLibrary.PrintString` NewItem))

(fn `AddItemToInventory`
  (params (NewItem :type "String (by ref)"))
  (`KismetArrayLibrary.Array_Add` (`self.Inventory`) NewItem)
  (`KismetSystemLibrary.PrintString` NewItem))

(fn `AddLureToInventory`
  (params (NewItem :type "String (by ref)"))
  (`KismetArrayLibrary.Array_Add` (`self.Lures`) NewItem)
  (`KismetSystemLibrary.PrintString` NewItem))

(fn `RemoveBaitsFromInventory`)

(fn `RemoveFishFromInventory`)