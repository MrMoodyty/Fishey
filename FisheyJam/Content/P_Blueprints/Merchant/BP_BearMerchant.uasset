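; Bear merchant NPC that runs a behavior tree and opens a shop state when the player interacts with it.
; Tick sets a WalkAround flag from its velocity.
; Interacting halts the bear, blends the camera to it, hides the player, switches to UI-only input with a cursor and sets ShopIsOpen.
; LookAt supplies the interaction prompt text; closing the shop is not handled here.
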(event `self.ReceiveTick`
  (params (DeltaSeconds :type "Float (single-precision)"))
  (if (> (`KismetMathLibrary.VSize` (`self.GetVelocity`)) 0.0)
    (set `self.WalkAround` true)
    (else
      (set `self.WalkAround` false))))

(event `self.ReceiveBeginPlay`
  (`AIController.RunBehaviorTree` (`AIBlueprintHelperLibrary.GetAIController` self) (`self.BTAsset`)))

(event `/Game/P_Blueprints/Inventory/I_InteractInterface.InteractWith`
  (params (PlayerCharacter :type "/Game/Tyler/BluePrints/ThirdPersonCharacter_BP Object Reference"))
  (bind _returnvalue (`GameplayStatics.GetPlayerController` 0))
  (if (== PlayerCharacter (`GameplayStatics.GetPlayerCharacter` 0))
    (`MovementComponent.StopMovementImmediately` (`self.CharacterMovement`))
    (`PlayerController.SetViewTargetWithBlend` (`GameplayStatics.GetPlayerController` 0) self 1.0 "VTBlend_Linear" 0.0 false)
    (`WidgetBlueprintLibrary.SetInputMode_UIOnlyEx` _returnvalue null)
    (set `PlayerController.bShowMouseCursor` true _returnvalue)
    (`self.SetActorHiddenInGame` (`GameplayStatics.GetPlayerCharacter` 0) true)
    (set `self.ShopIsOpen` true)))

(fn `LookAt`
  (returns (Message :type Text))
  (return "Interact with BEAR"))

(fn `UserConstructionScript`)